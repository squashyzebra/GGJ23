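; Collectable plant pickup actor that takes on the look of one plant Type: Acorn, Mandrake, Spring Onion, Snap Dragon or Radish.
; BeginPlay switches on Type to set the Cube mesh and material, using the Accessory mesh only for Acorn.
; The other types hide Accessory, rescale Cube (Snap Dragon also rotates it) and set its collision object type to Pawn.
; No pickup logic lives in these graphs.
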(event `self.ReceiveBeginPlay`
  (bind _cube (`self.Cube`))
  (bind _accessory (`self.Accessory`))
  (bind _cube_2 (`self.Cube`))
  (bind _cube_3 (`self.Cube`))
  (switch `string` (`self.Type`)
    (:`Acorn`
      (`StaticMeshComponent.SetStaticMesh` _cube_2 "/Game/Assets/Acorn/a_corn__Sphere.a_corn__Sphere")
      (`StaticMeshComponent.SetStaticMesh` _accessory "/Game/Assets/Acorn/a_corn__Sphere_001.a_corn__Sphere_001")
      (`PrimitiveComponent.SetMaterial` _cube_2 0 "/Game/Assets/Acorn/Material_006.Material_006")
      (`PrimitiveComponent.SetMaterial` _accessory 0 "/Game/Assets/Acorn/Material_007.Material_007"))
    (:`Mandrake`
      (`StaticMeshComponent.SetStaticMesh` _cube_2 "/Game/AllThemAssets/Characters/RoseHip/StaticMesh.StaticMesh")
      (`PrimitiveComponent.SetMaterial` _cube_2 0 "/Game/AllThemAssets/Characters/RoseHip/NewMaterial.NewMaterial")
      (`SceneComponent.SetVisibility` (`self.Accessory`) false false)
      (`SceneComponent.SetRelativeScale3D` (`self.Cube`) (0.125 0.125 0.125))
      (`PrimitiveComponent.SetCollisionObjectType` (`self.Cube`) "ECC_Pawn" :!label _label))
    (:`SpringOnion`
      (`StaticMeshComponent.SetStaticMesh` _cube_2 "/Game/AllThemAssets/Characters/SpringOnion/StaticMeshOnion.StaticMeshOnion")
      (`PrimitiveComponent.SetMaterial` _cube_2 0 "/Game/AllThemAssets/Characters/SpringOnion/lambert1.lambert1")
      (`SceneComponent.SetVisibility` (`self.Accessory`) false false)
      (`SceneComponent.SetRelativeScale3D` (`self.Cube`) (0.1875 0.1875 0.1875))
      (goto _label))
    (:`SnapDragon`
      (`StaticMeshComponent.SetStaticMesh` _cube_3 "/Game/AllThemAssets/Characters/sNP_TBD/StaticMesh.StaticMesh")
      (`PrimitiveComponent.SetMaterial` _cube_3 0 "/Game/AllThemAssets/Characters/sNP_TBD/defaultMat.defaultMat")
      (`SceneComponent.SetVisibility` (`self.Accessory`) false false)
      (`SceneComponent.SetRelativeScale3D` (`self.Cube`) (9.875 9.875 9.875))
      (`SceneComponent.K2_SetRelativeRotation` (`self.Cube`) (struct :`Roll` 90.0) false false)
      (goto _label))
    (:`Radish`
      (`StaticMeshComponent.SetStaticMesh` _cube "/Game/AllThemAssets/Characters/Radish/StaticMesh.StaticMesh")
      (`PrimitiveComponent.SetMaterial` _cube 0 "/Game/AllThemAssets/Characters/Radish/Textures/Radish.Radish")
      (`SceneComponent.SetVisibility` (`self.Accessory`) false false)
      (`SceneComponent.SetRelativeScale3D` (`self.Cube`) (0.1875 0.1875 0.1875))
      (goto _label))))

(fn `UserConstructionScript`)