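; BP_DayNight is a day/night cycle timer that tracks whether it is currently day through the IsDay flag.
; Tick accumulates delta seconds into Timer and compares it with DayTime or NightTime, depending on the current phase.
; When the phase's duration is reached, it flips IsDay and resets Timer to zero.
; It only maintains this state and applies no lighting or other effects itself.
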(event `self.ReceiveTick`
  (params (DeltaSeconds :type "Float (single-precision)"))
  (bind _timer (`self.Timer`))
  ;[1 1 1] increment timer
  (set `self.Timer` (+ DeltaSeconds (`self.Timer`)))
  (if (`self.isDay`)
    (if (not (> (`self.DayTime`) _timer))
      (set `self.isDay` false)
      (set `self.Timer` 0.0 :!label _label))
    (elif (not (> (`self.NightTime`) _timer))
      (set `self.isDay` true)
      (goto _label))))

(fn `UserConstructionScript`)