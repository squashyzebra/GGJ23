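; BP_Mandrake is a support plant that heals attack plants around it.
; BeginPlay sets its own health.
; Tick gathers every BP_AttackPlant and passes through a Delay, which turns the per-frame event into a repeating pulse every few seconds.
; Each pulse adds health to plants within range, with no maximum check, then spawns an attached Niagara effect.
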(event `self.ReceiveBeginPlay`
  (`parent.ReceiveBeginPlay`)
  (bind _output_get (set `self.maxHealth` 600.0))
  (set `self.health` _output_get))

(event `self.ReceiveTick`
  (params (DeltaSeconds :type "Float (single-precision)"))
  (`parent.ReceiveTick` DeltaSeconds)
  (bind _outactors (`GameplayStatics.GetAllActorsOfClass` "/Game/BluePrints/Plants/Fruits/BP_AttackPlant.BP_AttackPlant_C"))
  (`KismetSystemLibrary.Delay` 3.0)
  (for _array_element _outactors
    (if (< (`self.GetDistanceTo` _array_element) 1000.0)
      (set `/Game/BluePrints/Plants/BP_BasePlant.health` (+ (`/Game/BluePrints/Plants/BP_BasePlant.health` _array_element) 10.0) _array_element)))
  (`NiagaraFunctionLibrary.SpawnSystemAttached` "/Game/Assets/mandrake/NewNiagaraSystem.NewNiagaraSystem" (`self.Niagara`) "None" (0.0 0.0 0.0) (struct) "KeepRelativeOffset" true))

(fn `UserConstructionScript`
  (`parent.UserConstructionScript`))