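; BP_LastPlant is a high-health fruit plant that damages enemies in front of it.
; BeginPlay sets its health and range.
; Tick gathers all farm plots each frame, and a Delay throttles the attack to roughly twice a second.
; A forward line trace from Eyes ignores those plots and subtracts health directly from any BP_Enemy it hits; Bite is empty.
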(event `self.ReceiveBeginPlay`
  (`parent.ReceiveBeginPlay`)
  (bind _output_get (set `self.maxHealth` 1500.0))
  (set `self.health` _output_get)
  (set `self.range` 500.0))

(event `self.ReceiveTick`
  (params (DeltaSeconds :type "Float (single-precision)"))
  (bind _range (`self.range`))
  (bind _returnvalue (`SceneComponent.K2_GetComponentLocation` (`self.Eyes`)))
  (`parent.ReceiveTick` DeltaSeconds)
  (bind _outactors (`GameplayStatics.GetAllActorsOfClass` "/Game/BluePrints/Farming/BP_FarmPlot.BP_FarmPlot_C"))
  (`KismetSystemLibrary.Delay` 0.5)
  (bind (_outhit _returnvalue_2) (`KismetSystemLibrary.LineTraceSingle` _returnvalue (+ _returnvalue (* (`KismetMathLibrary.GetForwardVector` (`self.K2_GetActorRotation`)) (`KismetMathLibrary.MakeVector` _range _range _range))) "TraceTypeQuery1" false _outactors))
  (if _returnvalue_2
    (bind _asbp_enemy (cast `/Game/BluePrints/Enemys/BP_Enemy` (`.HitActor` (`GameplayStatics.BreakHitResult` _outhit))))
    (set `/Game/BluePrints/Enemys/BP_Enemy.Health` (- (`/Game/BluePrints/Enemys/BP_Enemy.Health` _asbp_enemy) 15.0) _asbp_enemy)))

(fn `Bite`)

(fn `UserConstructionScript`
  (`parent.UserConstructionScript`))