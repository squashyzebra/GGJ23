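; BP_AttackPlant is a plant actor that finds and faces enemies.
; Each Tick it gathers all BP_Enemy actors and loops until one is within Range, using a distance check that also yaws the plant toward that enemy.
; CurrentTarget is set to the last enemy visited, even if none was in range, or cleared when no enemies exist.
; No attack logic appears in these graphs.
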(event `self.ReceiveTick`
  (params (DeltaSeconds :type "Float (single-precision)"))
  (`parent.ReceiveTick` DeltaSeconds)
  (bind _outactors (`GameplayStatics.GetAllActorsOfClass` "/Game/BluePrints/Enemys/BP_Enemy.BP_Enemy_C"))
  (if (`KismetArrayLibrary.Array_IsNotEmpty` _outactors)
    (for _array_element _outactors
      (bind _isinrange (`self.Is It In Range?` (`self.range`) _array_element))
      (if _isinrange
        (break)))
    (set `self.Current Target` _array_element)
    (else
      (set `self.Current Target` null))))

(fn `Is It In Range?`
  (params (Range :type "Float (double-precision)") (OtherActor :type "Actor Object Reference"))
  (returns (IsInRange :type Boolean))
  (bind (_returnvalue_roll _returnvalue_pitch _returnvalue_yaw) (`KismetMathLibrary.BreakRotator` (`KismetMathLibrary.FindLookAtRotation` (`self.K2_GetActorLocation`) (`self.K2_GetActorLocation` OtherActor))))
  (bind _returnvalue (> Range (`self.GetDistanceTo` OtherActor)))
  (if _returnvalue
    (`self.K2_SetActorRotation` (`KismetMathLibrary.MakeRotator` 0.0 0.0 _returnvalue_yaw))
    (return _returnvalue)
    (else
      (return _returnvalue))))

(fn `UserConstructionScript`
  (`parent.UserConstructionScript`))