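; BP_DropPlant is a plant Actor that grows to maturity, then repeatedly drops fruit.
; It starts tiny, and Tick accumulates Age to scale it uniformly toward full size at TimeToMature.
; Once mature, Tick sets IsMature and feeds a FruitGrowthTime Delay, which paces recurring DropFruit calls.
; DropFruit spawns the Drop class above the plant at a random horizontal offset.
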(event `self.ReceiveBeginPlay`
  (`parent.ReceiveBeginPlay`)
  (`self.SetActorScale3D` (0.01 0.01 0.01)))

(event `self.ReceiveTick`
  (params (DeltaSeconds :type "Float (single-precision)"))
  (bind _timetomature (`self.timeToMature`))
  (`parent.ReceiveTick` DeltaSeconds)
  (bind _output_get (set `self.age` (+ DeltaSeconds (`self.age`))))
  (if (> _output_get _timetomature)
    (`self.mature`)
    (`KismetSystemLibrary.Delay` (`self.fruitGrowthTime`))
    (`self.dropFruit`)
    (else
      (`self.SetActorScale3D` (* (/ _output_get _timetomature) (1.0 1.0 1.0))))))

(fn `dropFruit`
  (bind _returnvalue (`self.GetTransform`))
  (`|SpawnActorFromClass` (`self.drop`) (`KismetMathLibrary.MakeTransform` (`KismetMathLibrary.MakeVector` (+ (- (* (`KismetMathLibrary.RandomFloat`) 200.0) 100.0) (.x (.location _returnvalue))) (+ (.y (.location _returnvalue)) (- (* (`KismetMathLibrary.RandomFloat`) 200.0) 100.0)) (+ (.z (.location _returnvalue)) 200.0))) "Undefined" "OverrideRootScale" null null))

(fn `mature`
  (set `self.isMature` true))

(fn `UserConstructionScript`
  (`parent.UserConstructionScript`))