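; BP_AcornPlant is a vegetable plant that automatically fires acorn projectiles straight ahead.
; BeginPlay sets its health and firing range.
; Tick runs through a one-second Delay, so roughly once a second it spawns a BP_AcornProjectile at the Eyes component, passing the actor location and a point Range units along its forward vector as start and target.
; It does no enemy detection, and MakeReady is empty.
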(event `self.ReceiveBeginPlay`
  (`parent.ReceiveBeginPlay`)
  (bind _output_get (set `self.maxHealth` 750.0))
  (set `self.health` _output_get)
  (set `self.range` 500.0))

(event `self.ReceiveTick`
  (params (DeltaSeconds :type "Float (single-precision)"))
  (bind (_returnvalue_location _returnvalue_rotation) (`KismetMathLibrary.BreakTransform` (`self.GetTransform`)))
  (bind _range (`self.range`))
  (`parent.ReceiveTick` DeltaSeconds)
  (`KismetSystemLibrary.Delay` 1.0)
  (`|SpawnActorFromClass` "/Game/BluePrints/Plants/Vegetables/BP_AcornProjectile.BP_AcornProjectile_C" (`KismetMathLibrary.MakeTransform` (`SceneComponent.K2_GetComponentLocation` (`self.Eyes`)) _returnvalue_rotation) "AlwaysSpawn" "OverrideRootScale" null _returnvalue_location (+ _returnvalue_location (* (`KismetMathLibrary.GetForwardVector` (`self.K2_GetActorRotation`)) (`KismetMathLibrary.MakeVector` _range _range _range))) null))

(fn `makeReady`)

(fn `UserConstructionScript`
  (`parent.UserConstructionScript`))