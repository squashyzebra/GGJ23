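; Vegetable plant actor that grows to maturity, then drops a spawned item and destroys itself.
; Tick accumulates age and scales the plant up linearly until TimeToMature, then calls Mature to set IsMature and waits GrowthTime.
; DropFruit spawns the Drop class at the plant's transform and launches its Sphere upward within a randomized cone using DropForce before destroying the plant.
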(event `self.ReceiveBeginPlay`)

(event `self.ReceiveTick`
  (params (DeltaSeconds :type "Float (single-precision)"))
  (bind _timetomature (`self.timeToMature`))
  (bind _output_get (set `self.age` (+ DeltaSeconds (`self.age`))))
  (if (> _output_get _timetomature)
    (`self.mature`)
    (`KismetSystemLibrary.Delay` (`self.growthTime`))
    (`self.dropFruit`)
    (else
      (`self.SetActorScale3D` (* (/ _output_get _timetomature) (1.0 1.0 1.0))))))

(fn `dropFruit`
  (bind _returnvalue (`|SpawnActorFromClass` (`self.drop`) (`self.GetTransform`) "Undefined" "OverrideRootScale" null null))
  (`PrimitiveComponent.AddImpulse` (`/Game/BluePrints/Plants/BP_Fruit.Sphere` _returnvalue) (* (`KismetMathLibrary.RandomUnitVectorInConeInDegrees` (0.0 0.0 1.0) (* (`KismetMathLibrary.RandomFloat`) 45.0)) (`self.dropForce`)) "None" false)
  (`self.K2_DestroyActor`))

(fn `mature`
  (set `self.isMature` true))

(fn `UserConstructionScript`)