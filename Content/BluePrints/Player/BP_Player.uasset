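; Player character that moves, looks, jumps and plants seeds from a counted inventory onto farm plots.
; Interact line-traces from the Eyes along control rotation, and on a free BP_FarmPlot spawns the selected plant, decrements its count and occupies the plot.
; The ChangePlant axis cycles through Inventory map keys with wraparound, while AddItemToArray increments counts.
; Each plant type has its own collapsed spawn graph, though all currently spawn BP_BasePlant.
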(event `InputAxis|Forward`
  (params (AxisValue :type "Float (single-precision)"))
  ;[1 1 1] movement
  (`self.AddMovementInput` (`self.GetActorForwardVector`) AxisValue))

(event `InputAxis|Right`
  (params (AxisValue :type "Float (single-precision)"))
  ;[1 1 1] movement
  (`self.AddMovementInput` (`self.GetActorRightVector`) AxisValue))

(event `InputAction|Interact`
  (params (Key :type "Key Structure"))
  (bind _inventory (`self.Inventory`))
  (bind _currentplant (`self.CurrentPlant`))
  (bind _returnvalue (`SceneComponent.K2_GetComponentLocation` (`self.Eyes`)))
  ;[1 1 1] Interact
  (:`Pressed`
    (bind _outhit (`KismetSystemLibrary.LineTraceSingleForObjects` :`Start` _returnvalue :`End` (+ _returnvalue (* (`KismetMathLibrary.GetForwardVector` (`self.GetControlRotation`)) (500.0 500.0 500.0))) :`ObjectTypes` (`self.Object Types`) :`DrawDebugType` "ForDuration"))
    (if (`GameplayStatics.BreakHitResult` _outhit)
      (bind _asbp_farm_plot (cast `/Game/BluePrints/Farming/BP_FarmPlot` (`.HitActor` (`GameplayStatics.BreakHitResult` _outhit))))
      (if (and (not (== (`BlueprintMapLibrary.Map_Find` (`self.Inventory`) (`self.CurrentPlant`)) 0)) (`/Game/BluePrints/Farming/BP_FarmPlot.FreePlot` _asbp_farm_plot))
        ;[1 1 1] Placing plants
        (switch `string` (`self.CurrentPlant`)
          (:`Snapdragon`
            (bind _returnvalue_2 (`SceneComponent.K2_GetComponentLocation` (`.HitComponent` (`GameplayStatics.BreakHitResult` _outhit))))
            (`|SpawnActorFromClass` "/Game/BluePrints/Plants/BP_BasePlant.BP_BasePlant_C" (`KismetMathLibrary.MakeTransform` _returnvalue_2) "AlwaysSpawn" "OverrideRootScale" null null))
          (:`Pomegrenade`
            (`|SpawnActorFromClass` "/Game/BluePrints/Plants/BP_BasePlant.BP_BasePlant_C" (`KismetMathLibrary.MakeTransform` _returnvalue_2) "AlwaysSpawn" "OverrideRootScale" null null))
          (:`acorn`
            (`|SpawnActorFromClass` "/Game/BluePrints/Plants/BP_BasePlant.BP_BasePlant_C" (`KismetMathLibrary.MakeTransform` _returnvalue_2) "AlwaysSpawn" "OverrideRootScale" null null))
          (:`test4`
            (`|SpawnActorFromClass` "/Game/BluePrints/Plants/BP_BasePlant.BP_BasePlant_C" (`KismetMathLibrary.MakeTransform` _returnvalue_2) "AlwaysSpawn" "OverrideRootScale" null null))
          (:`test5`
            (`|SpawnActorFromClass` "/Game/BluePrints/Plants/BP_BasePlant.BP_BasePlant_C" (`KismetMathLibrary.MakeTransform` _returnvalue_2) "AlwaysSpawn" "OverrideRootScale" null null))
          (:`test6`
            (`|SpawnActorFromClass` "/Game/BluePrints/Plants/BP_BasePlant.BP_BasePlant_C" (`KismetMathLibrary.MakeTransform` _returnvalue_2) "AlwaysSpawn" "OverrideRootScale" null null))
          (:`test7`
            (`|SpawnActorFromClass` "/Game/BluePrints/Plants/BP_BasePlant.BP_BasePlant_C" (`KismetMathLibrary.MakeTransform` _returnvalue_2) "AlwaysSpawn" "OverrideRootScale" null null)))
        (bind _result (`/Engine/EditorBlueprintResources/StandardMacros.DecrementInt` (`BlueprintMapLibrary.Map_Find` _inventory _currentplant))
          (:`  `
            (`BlueprintMapLibrary.Map_Add` _inventory _currentplant _result)
            (set `/Game/BluePrints/Farming/BP_FarmPlot.FreePlot` false _asbp_farm_plot)))))))

(event `InputAxis|Turn`
  (params (AxisValue :type "Float (single-precision)"))
  ;[1 1 1] movement
  (`self.AddControllerYawInput` AxisValue))

(event `InputAxis|LookUp`
  (params (AxisValue :type "Float (single-precision)"))
  ;[1 1 1] movement
  (`self.AddControllerPitchInput` AxisValue))

(event `InputAction|Jump`
  (params (Key :type "Key Structure"))
  ;[1 1 1] movement
  (:`Pressed`
    (`self.Jump`))
  (:`Released`
    (`self.StopJumping`)))

(event `InputAxis|ChangePlant`
  (params (AxisValue :type "Float (single-precision)"))
  ;[1 1 1] Change selected plant
  (bind _keys (`BlueprintMapLibrary.Map_Keys` (`self.Inventory`)))
  (bind _returnvalue (+ AxisValue (`KismetArrayLibrary.Array_Find` _keys (`self.CurrentPlant`))))
  (if (< _returnvalue 0.0)
    (bind _returnvalue_2 (`KismetArrayLibrary.Array_Length` _keys))
    (set `self.CurrentPlant` (`|GetArrayItem` _keys (- _returnvalue_2 1)))
    (elif (> _returnvalue (- _returnvalue_2 1))
      (set `self.CurrentPlant` (`|GetArrayItem` _keys))
      (else
        (set `self.CurrentPlant` (`|GetArrayItem` _keys (`KismetMathLibrary.FTrunc` _returnvalue)))))))

(fn `AddItemToArray`
  (params (NewItem :type "String (by ref)"))
  (bind _inventory (`self.Inventory`))
  (bind (_value _returnvalue) (`BlueprintMapLibrary.Map_Find` _inventory NewItem))
  (if _returnvalue
    (bind _result (`/Engine/EditorBlueprintResources/StandardMacros.IncrementInt` _value)
      (:`  `
        (`BlueprintMapLibrary.Map_Add` _inventory NewItem _result)))
    (else
      (`BlueprintMapLibrary.Map_Add` _inventory NewItem 1))))

(fn `UserConstructionScript`)