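; BP_Enemy is an enemy that walks toward the Portal and costs the player health if it gets there.
; Every Tick it searches all BP_AttackPlant actors and moves to the first one in close range, otherwise to the Portal, via SimpleMoveToActor.
; Tick also polls Health, playing a death sound and destroying the enemy at zero.
; Overlapping the Portal deducts BP_Player health, plays a breaking sound and destroys the enemy.
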(event `self.ReceiveBeginPlay`
  (bind _output_get (set `self.MaxHealth` 100.0))
  (set `self.Health` _output_get))

(event `self.ReceiveTick`
  (params (DeltaSeconds :type "Float (single-precision)"))
  (if (<= (`self.Health`) 0.0)
    (`GameplayStatics.PlaySound2D` "/Game/AllThemAssets/SFX/enemy_dies.enemy_dies" 0.6 1.0 0.0 null null)
    (`self.K2_DestroyActor`)
    (else
      (bind _outactors (`GameplayStatics.GetAllActorsOfClass` "/Game/BluePrints/Plants/Fruits/BP_AttackPlant.BP_AttackPlant_C"))
      (if (`KismetArrayLibrary.Array_IsNotEmpty` _outactors)
        (for _array_element _outactors
          (bind _returnvalue (< (`self.GetDistanceTo` _array_element) 400.0))
          (if _returnvalue
            (bind _output_get (set `self.Target Plant` _array_element))
            (`AIBlueprintHelperLibrary.SimpleMoveToActor` (`self.GetController`) _output_get)
            (break)))
        (if (not _returnvalue)
          (bind _returnvalue_2 (`GameplayStatics.GetActorOfClass` "/Game/BluePrints/Farming/Portal.Portal_C" :!label _label))
          (`AIBlueprintHelperLibrary.SimpleMoveToActor` (`self.GetController`) _returnvalue_2))
        (else
          (goto _label))))))

(event `self.ReceiveActorBeginOverlap`
  (params (OtherActor :type "Actor Object Reference"))
  (cast `/Game/BluePrints/Farming/Portal` OtherActor)
  (bind _asbp_player (cast `/Game/BluePrints/Player/BP_Player` (`GameplayStatics.GetPlayerPawn` 0)))
  (set `/Game/BluePrints/Player/BP_Player.Health` (- (`/Game/BluePrints/Player/BP_Player.Health` _asbp_player) 10.0) _asbp_player)
  (`GameplayStatics.PlaySound2D` "/Game/AllThemAssets/SFX/portal_breaks.portal_breaks" 1.0 1.0 0.0 null null)
  (`self.K2_DestroyActor`))

(fn `UserConstructionScript`)